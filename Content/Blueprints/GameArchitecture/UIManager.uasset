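; UIManager is an actor that switches the on-screen UI between the main menu and play mode and exposes basic video controls.
; On BeginPlay it shows the main menu, then caches the first player controller, which later owns the play UI.
; Each switch removes the current widget before creating and attaching the next, tracked in a single reference.
; Separate functions pause the media player or reopen and play it for replay.
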(event `self.ReceiveBeginPlay`
  (`self.SetUpMainMenuUI`)
  (`self.SetUpReferences`))

(fn `PauseVideo`
  (`MediaPlayer.Pause` (`self.MediaPlayer`)))

(fn `ReplayVideo`
  (bind _mediaplayer (`self.MediaPlayer`))
  (`MediaPlayer.Reopen` _mediaplayer)
  (`MediaPlayer.Play` _mediaplayer))

(fn `SetUpMainMenuUI`
  (bind _currentattachedwidget (`self.CurrentAttachedWidget`))
  (`/Engine/EditorBlueprintResources/StandardMacros.IsValid` _currentattachedwidget
    (:`Is Valid`
      (`Widget.RemoveFromParent` _currentattachedwidget))
    (:`Is Not Valid`
      _))
  (bind _returnvalue (`|CreateWidget` "/Game/Blueprints/Widgets/WBP_MainMenu.WBP_MainMenu_C"))
  (bind _output_get (set `self.CurrentAttachedWidget` _returnvalue))
  (`UserWidget.AddToViewport` _output_get 0))

(fn `SetUpPlayModeUI`
  (bind _currentattachedwidget (`self.CurrentAttachedWidget`))
  (`/Engine/EditorBlueprintResources/StandardMacros.IsValid` _currentattachedwidget
    (:`Is Valid`
      (`Widget.RemoveFromParent` _currentattachedwidget))
    (:`Is Not Valid`
      _))
  (bind _returnvalue (`|CreateWidget` "/Game/Blueprints/Widgets/WBP_PlayUI.WBP_PlayUI_C" (`self.PlayerController`)))
  (bind _output_get (set `self.CurrentAttachedWidget` _returnvalue))
  (`UserWidget.AddToViewport` _output_get 0))

(fn `SetUpReferences`
  (set `self.PlayerController` (`GameplayStatics.GetPlayerController` 0)))

(fn `UserConstructionScript`)